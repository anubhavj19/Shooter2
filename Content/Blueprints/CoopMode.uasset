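; CoopMode is a co-op mode Blueprint that drives enemy spawning and holds unused logic for spawning two local players.
; On BeginPlay it sets a looping timer that calls SpawnEnemy on the first EnemySpawner found, at a rate set by EnemiesPerSecond.
; GetPlayerStartPoints and SpawnPlayers would create, spawn and possess two hero characters by PlayerStart tag, but their calls in the event graph are disconnected.
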(event `self.ReceiveBeginPlay`
  (bind _outactors (`GameplayStatics.GetAllActorsOfClass` "/Game/Blueprints/enemySpawner.EnemySpawner_C"))
  (bind _output_get (set `self.Spawner` (`|GetArrayItem` _outactors)))
  (`KismetSystemLibrary.K2_SetTimer` _output_get "SpawnEnemy" (/ 1.0 (`self.EnemiesPerSecond`)) true))

(fn `GetPlayerStartPoints`
  (bind _outactors (`GameplayStatics.GetAllActorsOfClass` "/Script/Engine.PlayerStart"))
  (set `self.PlayerStartArray` _outactors))

(fn `SpawnPlayers`
  (for _array_element (`self.PlayerStartArray`)
    (if (== (`PlayerStart.PlayerStartTag` _array_element) "0")
      (`GameplayStatics.CreatePlayer` 0)
      (bind _returnvalue (`self.GetTransform` _array_element))
      (bind _returnvalue_2 (`|SpawnActorFromClass` "/Game/Blueprints/HeroCharacter_1.HeroCharacter_1_C" _returnvalue "AlwaysSpawn" "OverrideRootScale" null null))
      (`Controller.Possess` (`GameplayStatics.GetPlayerControllerFromID` 0) _returnvalue_2)
      (else
        (`GameplayStatics.CreatePlayer` 1)
        (bind _returnvalue_3 (`|SpawnActorFromClass` "/Game/Blueprints/HeroCharacter_2.HeroCharacter_2_C" _returnvalue "AlwaysSpawn" "OverrideRootScale" null null))
        (`Controller.Possess` (`GameplayStatics.GetPlayerControllerFromID` 1) _returnvalue_3)))))

(fn `UserConstructionScript`)