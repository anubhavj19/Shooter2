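; Player controller for two-player local twin-stick play that spawns both heroes and handles input for both.
; On BeginPlay it creates players at tagged PlayerStarts, possesses a hero for each and attaches a weapon to each GunTemp.
; Per-player axes drive world-aligned movement, while look input past a deadzone sets control rotation and holds the weapon trigger.
; SlowTime toggles global time dilation through a looping MultiGate.
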(event `self.ReceiveBeginPlay`
  (bind _returnvalue (`GameplayStatics.GetPlayerCharacter` 0))
  (bind _returnvalue_2 (`GameplayStatics.GetPlayerCharacter` 1))
  (`self.GetPlayerStartPoints`)
  (`self.SpawnPlayers`)
  ;[1 1 1] Spawning players and weapon configuration
  (`|ExecutionSequence`
    (:`then_0`
      (`/Engine/EditorBlueprintResources/StandardMacros.IsValid` _returnvalue
        (:`Is Valid`
          (bind _ashero_character_1 (cast `/Game/Blueprints/HeroCharacter_1` _returnvalue))
          (bind _guntemp (`/Game/Blueprints/HeroCharacter_1.GunTemp` _ashero_character_1))
          (bind _returnvalue_3 (`|SpawnActorFromClass` "/Game/Blueprints/Weapon.Weapon_C" (`KismetMathLibrary.Conv_VectorToTransform` (`SceneComponent.K2_GetComponentLocation` _guntemp)) "Undefined" "OverrideRootScale" null null))
          (bind _output_get (set `self.TempWeapon` _returnvalue_3))
          (`self.K2_AttachToComponent` _output_get _guntemp "None" "SnapToTarget" "KeepRelative" "KeepRelative" true))))
    (:`then_1`
      (`/Engine/EditorBlueprintResources/StandardMacros.IsValid` _returnvalue_2
        (:`Is Valid`
          (bind _ashero_character_2 (cast `/Game/Blueprints/HeroCharacter_2` _returnvalue_2))
          (bind _guntemp_2 (`/Game/Blueprints/HeroCharacter_2.GunTemp` _ashero_character_2))
          (bind _returnvalue_4 (`|SpawnActorFromClass` "/Game/Blueprints/Weapon.Weapon_C" (`SceneComponent.K2_GetComponentToWorld` _guntemp_2) "Undefined" "OverrideRootScale" null null))
          (`/Engine/EditorBlueprintResources/StandardMacros.IsValid` _returnvalue_4
            (:`Is Valid`
              (bind _output_get_2 (set `self.TempWeapon2` _returnvalue_4))
              (`self.K2_AttachToComponent` _output_get_2 _guntemp_2 "None" "SnapToTarget" "KeepRelative" "KeepRelative" true))))))))

(event `InputAxis|MoveUp1`
  (params (AxisValue :type "Float (single-precision)"))
  ;[1 1 1] P1Motion
  (`Pawn.AddMovementInput` (`GameplayStatics.GetPlayerPawn` 0) (1.0 0.0 0.0) AxisValue false))

(event `InputAxis|MoveRight1`
  (params (AxisValue :type "Float (single-precision)"))
  ;[1 1 1] P1Motion
  (`Pawn.AddMovementInput` (`GameplayStatics.GetPlayerPawn` 0) (0.0 1.0 0.0) AxisValue false))

(event `InputAxis|LookUp1`
  (params (AxisValue :type "Float (single-precision)"))
  (bind _tempweapon (`self.TempWeapon`))
  ;[1 1 1] P1Motion
  (bind _returnvalue (`KismetMathLibrary.MakeVector` AxisValue (stale `InputAxis|LookRight1` AxisValue)))
  (if (> (`KismetMathLibrary.VSize` _returnvalue) 0.25) :!label _label
    (`self.SetControlRotation` (`GameplayStatics.GetPlayerControllerFromID` 0) (`KismetMathLibrary.Conv_VectorToRotator` _returnvalue))
    ;[1 1 1] P1 Fire
    (`/Engine/EditorBlueprintResources/StandardMacros.IsValid` _tempweapon
      (:`Is Valid`
        (`/Game/Blueprints/Weapon.PullTrigger` _tempweapon)))
    (else
      (`/Engine/EditorBlueprintResources/StandardMacros.IsValid` _tempweapon
        (:`Is Valid`
          (`/Game/Blueprints/Weapon.ReleaseTrigger` _tempweapon))))))

(event `InputAxis|LookRight1`
  (params (AxisValue :type "Float (single-precision)"))
  ;[1 1 1] P1Motion
  (goto _label))

(event `InputAxis|MoveUp2`
  (params (AxisValue :type "Float (single-precision)"))
  ;[1 1 1] P2Motion
  (`Pawn.AddMovementInput` (`GameplayStatics.GetPlayerPawn` 1) (1.0 0.0 0.0) AxisValue false))

(event `InputAxis|MoveRight2`
  (params (AxisValue :type "Float (single-precision)"))
  ;[1 1 1] P2Motion
  (`Pawn.AddMovementInput` (`GameplayStatics.GetPlayerPawn` 1) (0.0 1.0 0.0) AxisValue false))

(event `InputAxis|LookUp2`
  (params (AxisValue :type "Float (single-precision)"))
  (bind _tempweapon2 (`self.TempWeapon2`))
  ;[1 1 1] P2Motion
  (bind _returnvalue (`KismetMathLibrary.MakeVector` AxisValue (stale `InputAxis|LookRight2` AxisValue)))
  (if (> (`KismetMathLibrary.VSize` _returnvalue) 0.25) :!label _label_2
    (`self.SetControlRotation` (`GameplayStatics.GetPlayerControllerFromID` 1) (`KismetMathLibrary.Conv_VectorToRotator` _returnvalue))
    ;[1 1 1] P2 Fire
    (`/Engine/EditorBlueprintResources/StandardMacros.IsValid` _tempweapon2
      (:`Is Valid`
        (`/Game/Blueprints/Weapon.PullTrigger` _tempweapon2)))
    (else
      (`/Engine/EditorBlueprintResources/StandardMacros.IsValid` _tempweapon2
        (:`Is Valid`
          (`/Game/Blueprints/Weapon.ReleaseTrigger` _tempweapon2))))))

(event `InputAxis|LookRight2`
  (params (AxisValue :type "Float (single-precision)"))
  ;[1 1 1] P2Motion
  (goto _label_2))

(event `InputAction|SlowTime`
  (params (Key :type "Key Structure"))
  (bind _timedilation (`self.TimeDilation`))
  ;[1 1 1] TimeDilation
  (:`Pressed`
    (`|MultiGate` false true
      (:`Out 0`
        (`GameplayStatics.SetGlobalTimeDilation` _timedilation)
        (`KismetSystemLibrary.PrintString` (`KismetStringLibrary.Conv_DoubleToString` _timedilation)))
      (:`Out 1`
        (`GameplayStatics.SetGlobalTimeDilation` 1.0)))))

(fn `GetPlayerStartPoints`
  (bind _outactors (`GameplayStatics.GetAllActorsOfClass` "/Script/Engine.PlayerStart"))
  (set `self.PlayerStartArray` _outactors))

(fn `SpawnPlayers`
  (bind _returnvalue (`GameplayStatics.GetPlayerControllerFromID` 1))
  (bind _returnvalue_2 (`GameplayStatics.GetPlayerControllerFromID` 0))
  (for _array_element (`self.PlayerStartArray`)
    (if (== (`PlayerStart.PlayerStartTag` _array_element) "0")
      (`GameplayStatics.CreatePlayer` 0)
      (bind _returnvalue_3 (`self.GetTransform` _array_element))
      (bind _returnvalue_4 (`|SpawnActorFromClass` "/Game/Blueprints/HeroCharacter_1.HeroCharacter_1_C" _returnvalue_3 "Undefined" "OverrideRootScale" null null))
      (`/Engine/EditorBlueprintResources/StandardMacros.IsValid` _returnvalue_2
        (:`Is Valid`
          (`self.Possess` _returnvalue_2 _returnvalue_4)))
      (else
        (`GameplayStatics.CreatePlayer` 1)
        (bind _returnvalue_5 (`|SpawnActorFromClass` "/Game/Blueprints/HeroCharacter_2.HeroCharacter_2_C" _returnvalue_3 "Undefined" "OverrideRootScale" null null))
        (`/Engine/EditorBlueprintResources/StandardMacros.IsValid` _returnvalue
          (:`Is Valid`
            (`self.Possess` _returnvalue _returnvalue_5)))))))

(fn `UserConstructionScript`)