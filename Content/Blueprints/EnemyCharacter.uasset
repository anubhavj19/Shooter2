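; EnemyCharacter is an enemy Blueprint that takes health changes and removes itself when dead.
; AffectHealth passes the delta to CalculateHealth, then, if IsDead, destroys each attached actor.
; The self-destroy call sits inside that loop, so it only runs when at least one actor is attached.
; The construction script creates a dynamic material instance on the mesh and sets its BodyColor to black.
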(event `/Game/Blueprints/iDamageable.AffectHealth`
  (params (Delta :type "Float (single-precision)"))
  (`self.CalculateHealth` Delta)
  (if (`self.isDead`)
    (for _array_element (`self.GetAttachedActors` true)
      (`self.K2_DestroyActor` _array_element)
      (`self.K2_DestroyActor`))))

(fn `UserConstructionScript`
  (bind _returnvalue (`PrimitiveComponent.CreateDynamicMaterialInstance` (`self.Mesh`) 0 null "None"))
  (bind _output_get (set `self.DynaMat` _returnvalue))
  (`MaterialInstanceDynamic.SetVectorParameterValue` _output_get "BodyColor" (struct :`A` 1.0)))