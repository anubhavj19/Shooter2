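; Enemy spawner Blueprint that creates armed AI enemies at random points inside its SpawnVolume.
; SpawnEnemy spawns an EnemyCharacter running EnemyBT, then spawns a Weapon owned by it and attaches it to the GunHolder.
; A looping timer calls the weapon's Fire function by name at a fixed interval, so firing is set up here by the spawner.
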(event `SpawnEnemy`
  (bind _spawnvolume (`self.SpawnVolume`))
  (bind _returnvalue (`AIBlueprintHelperLibrary.SpawnAIFromClass` "/Game/Blueprints/EnemyCharacter.EnemyCharacter_C" "/Game/AI/EnemyBT.EnemyBT" (`KismetMathLibrary.RandomPointInBoundingBox` (`SceneComponent.K2_GetComponentLocation` _spawnvolume) (`BoxComponent.GetScaledBoxExtent` _spawnvolume))))
  (bind _output_get (set `self.BotEnemy` _returnvalue))
  (bind _asenemy_character (cast `/Game/Blueprints/EnemyCharacter` _output_get))
  (bind _gunholder (`/Game/Blueprints/EnemyCharacter.GunHolder` _asenemy_character))
  (bind _returnvalue_2 (`|SpawnActorFromClass` "/Game/Blueprints/Weapon.Weapon_C" (`SceneComponent.K2_GetComponentToWorld` _gunholder) "Undefined" "OverrideRootScale" _asenemy_character null))
  (bind _output_get_2 (set `self.GunSocket` _returnvalue_2))
  (`self.K2_AttachToComponent` _output_get_2 _gunholder "None" "SnapToTarget" "KeepRelative" "KeepRelative" true)
  (`KismetSystemLibrary.K2_SetTimer` (`self.GunSocket`) "Fire" 3.0 true))

(fn `UserConstructionScript`)